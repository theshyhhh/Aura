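; BP_FireBall is a projectile actor for the Aura Fire Blast ability that flies out and returns to its instigator.
; On the server, an outgoing timeline lerps it along its forward vector to a set travel distance, then a return timeline lerps it toward the instigator's current location.
; Once within explode distance of the instigator, it triggers its hit handling, causes explosion damage and destroys itself.
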(event EventStartOutgoingTimeline
  (Networking|SwitchHasAuthority
    (:Authority
      (Variables|Default|SetInitialLocation (Transformation|GetActorLocation))
      (Variables|Default|SetFurthestLocation (+ (Variables|Default|GetInitialLocation) (* (Transformation|GetActorForwardVector) (Variables|Default|GetTravelDistance))))
      (bind _outgoingtrack (Timeline|OutgoingTimeline PlayFromStart)
        (:Update
          (Transformation|SetActorLocation (Math|Vector|Lerp(Vector) (Variables|Default|GetInitialLocation) (Variables|Default|GetFurthestLocation) _outgoingtrack) false false))
        (:Finished
          (bind _returntrack (Timeline|ReturnTimeline PlayFromStart)
            (:Update
              (Transformation|SetActorLocation (Math|Vector|Lerp(Vector) (Variables|Default|GetFurthestLocation) (Transformation|GetActorLocation (Game|GetInstigator)) _returntrack) false false)
              (if (CallFunction|IsWithinExplodeDistance)
                (Class|AuraProjectile|OnHit)
                (Class|AuraFireBall|CauseExplosionDamage)
                (Actor|DestroyActor)))))))))

(fn ConstructionScript)

(fn IsWithinExplodeDistance
  (return (< (Math|Vector|VectorLength (- (Transformation|GetActorLocation) (Transformation|GetActorLocation (Game|GetInstigator)))) (Variables|Default|GetExplodeDistance))))