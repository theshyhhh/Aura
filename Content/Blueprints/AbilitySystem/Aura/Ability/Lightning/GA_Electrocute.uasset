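; Channeled Electrocute lightning ability that locks movement and beams from the weapon tip toward the cursor hit, chaining to additional targets.
; A montage event starts the trace and ShockLoop cues, then a looping timer commits cost and damages targets, or only drains cost without a combat target.
; Input release (after a minimum hold), failed cost or primary target death ends it with cooldown.
; Release and failed damage ticks also apply debuffs server-side.
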(event Custom|CommitCost
  (bind _returnvalue (Ability|CommitAbilityCost false))
  (if (not _returnvalue)
    (Ability|CommitAbilityCooldown false)
    (Ability|EndAbility)))

(event Custom|DamageAndCost
  (bind _returnvalue (Ability|CommitAbilityCost false))
  (if _returnvalue
    (CallFunction|ApplyDamage)
    (else
      (CallFunction|ApplyDebuff)
      (Ability|CommitAbilityCooldown false)
      (Ability|EndAbility))))

(event Ability|EventActivateAbility
  (bind _data (|TargetDataUnderMouse)
    (:ValidData
      (Class|AuraBeamSpell|SetMouseHitInfo (Ability|TargetData|GetHitResultfromTargetData _data))
      (Utilities|FlowControl|Sequence
        (:then_0
          (Variables|/Script/Engine.PlayerController|SetbShowMouseCursor (Class|AuraBeamSpell|GetOwnerController) false)
          (Class|CombatInterface|SetFacingTarget(Message) (Ability|GetAvatarActorfromActorInfo) (Variables|Default|GetMouseHitLocation))
          (GameplayCue|ExecuteGameplayCue :GameplayCueTag "(TagName=\"GameplayCue.ShockBurst\")")
          (|PlayMontageandWaitProxy "None" (Variables|AuraBeamSpell|GetMontage_Electrocute) 1.0 "None" true 1.0 0.0 false
            (:then
              (Ability|Tasks|WaitGameplayEvent "(TagName=\"Event.Montage.Electrocute\")" 0
                (:EventReceived
                  (Class|CombatInterface|SetinShockLoop(Message) (Ability|GetAvatarActorfromActorInfo) true)
                  (Pawn|Components|CharacterMovement|DisableMovement (Variables|/Script/Engine.Character|GetCharacterMovement (Class|AuraBeamSpell|GetOwnerCharacter)))
                  (bind _returnvalue (Class|CombatInterface|GetWeaponMesh(Message) (Ability|GetAvatarActorfromActorInfo)))
                  (Variables|Default|SetOwnerWeaponMesh _returnvalue)
                  (Class|AuraBeamSpell|TraceFirstTarget (Transformation|GetSocketLocation (Variables|Default|GetOwnerWeaponMesh) "TipSocket") (Variables|Default|GetMouseHitLocation))
                  (Variables|Electrocute|SetFirstTraceCueParams (Ability|GameplayCue|MakeGameplayCueParameters :Location (Variables|Default|GetMouseHitLocation) :SourceObject (Variables|Default|GetHitActor) :TargetAttachComponent (Variables|Default|GetOwnerWeaponMesh)))
                  (if (Utilities|DoesObjectImplementInterface (Variables|Default|GetHitActor) "/Script/Aura.CombatInterface")
                    (Variables|Electrocute|SetTargetToAddCue (Variables|Default|GetHitActor))
                    (GameplayCue|AddGameplayCueOnActor(Looping) (Variables|Electrocute|GetTargetToAddCue) "(TagName=\"GameplayCue.ShockLoop\")" (Variables|Electrocute|GetFirstTraceCueParams))
                    (Class|CombatInterface|SetIsBeingElectrocuted(Message) (Variables|Electrocute|GetTargetToAddCue) true)
                    (bind _outadditionalactors (Class|AuraBeamSpell|StoreAdditionalTarget))
                    (bind _output_get (Variables|Electrocute|SetAdditional%20Actors _outadditionalactors))
                    (for _array_element _output_get
                      (CallFunction|AddGameplayCuetoAddtionalActor _array_element)
                      (Class|CombatInterface|SetIsBeingElectrocuted(Message) _array_element true))
                    (bind _returnvalue_2 (Utilities|Time|SetTimerbyEvent (delegate Custom|DamageAndCost) (Variables|Default|GetDamageDeltaTime) true))
                    (Variables|Default|SetDamageAndCostTimer _returnvalue_2)
                    (else
                      (Variables|Electrocute|SetTargetToAddCue (Ability|GetAvatarActorfromActorInfo))
                      (GameplayCue|AddGameplayCueOnActor(Looping) (Variables|Electrocute|GetTargetToAddCue) "(TagName=\"GameplayCue.ShockLoop\")" (Variables|Electrocute|GetFirstTraceCueParams))
                      (bind _returnvalue_3 (Utilities|Time|SetTimerbyEvent (delegate Custom|CommitCost) (Variables|Default|GetDamageDeltaTime) true))
                      (Variables|Default|SetDamageAndCostTimer _returnvalue_3))))))))
        (:then_1
          (bind _timeheld (Ability|Tasks|WaitInputRelease false)
            (:OnRelease
              (bind _output_get_2 (Variables|Default|SetTime%20Held _timeheld))
              (if (> _output_get_2 (Variables|Default|GetMinSpellTime))
                _
                (else
                  (Utilities|FlowControl|Delay (- (Variables|Default|GetMinSpellTime) (Variables|Default|GetTime%20Held)))))
              (CallFunction|ApplyDebuff)
              (Ability|CommitAbilityCooldown false)
              (Ability|EndAbility))))))))

(event Ability|EventOnEndAbility
  (params (bWasCancelled :type Boolean))
  (Utilities|Time|ClearandInvalidateTimerbyHandle (Variables|Default|GetDamageAndCostTimer))
  (Variables|/Script/Engine.PlayerController|SetbShowMouseCursor (Class|AuraBeamSpell|GetOwnerController) true)
  (Class|CombatInterface|SetinShockLoop(Message) (Ability|GetAvatarActorfromActorInfo) false)
  (Pawn|Components|CharacterMovement|SetMovementMode (Variables|/Script/Engine.Character|GetCharacterMovement (Class|AuraBeamSpell|GetOwnerCharacter)) "MOVE_Walking" 0)
  (GameplayCue|RemoveGameplayCueOnActor(Looping) (Variables|Electrocute|GetTargetToAddCue) "(TagName=\"GameplayCue.ShockLoop\")" (Variables|Electrocute|GetFirstTraceCueParams))
  (Class|CombatInterface|SetIsBeingElectrocuted(Message) (Variables|Electrocute|GetTargetToAddCue) false)
  (for _array_element (Variables|Electrocute|GetAdditional%20Actors)
    (CallFunction|RemoveGameplayCuefromAddtionalActor _array_element)
    (Class|CombatInterface|SetIsBeingElectrocuted(Message) _array_element false))
  (Utilities|Map|Clear (Variables|Electrocute|GetAddtionalActorToGCParams))
  (Utilities|Array|Clear (Variables|Electrocute|GetAdditional%20Actors)))

(event EventOnPrimaryTargetDeath
  (params (DeadActor :type Actor%20Object%20Reference))
  (Ability|CommitAbilityCooldown false)
  (Ability|EndAbility))

(event EventOnAdditionalTargetDeath
  (params (DeadActor :type Actor%20Object%20Reference))
  (GameplayCue|RemoveGameplayCueOnActor(Looping) DeadActor "(TagName=\"GameplayCue.ShockLoop\")" (.Value (Utilities|Map|Find (Variables|Electrocute|GetAddtionalActorToGCParams) DeadActor)))
  (Utilities|Array|RemoveItem (Variables|Electrocute|GetAdditional%20Actors) DeadActor)
  (Utilities|Map|Remove (Variables|Electrocute|GetAddtionalActorToGCParams) DeadActor))

(fn AddGameplayCuetoAddtionalActor
  (params (Actor :type Actor%20Object%20Reference%20%28by%20ref%29))
  (LocalVariables|SetLocalActor Actor)
  (LocalVariables|SetGCParams (Ability|GameplayCue|MakeGameplayCueParameters :Location (+ (Transformation|GetActorLocation (LocalVariables|GetLocalActor)) "0.000000,0.000000,20.000000") :SourceObject (LocalVariables|GetLocalActor) :TargetAttachComponent (Variables|/Script/Engine.Actor|GetRootComponent (Variables|Default|GetHitActor))))
  (Utilities|Map|Add (Variables|Electrocute|GetAddtionalActorToGCParams) (LocalVariables|GetLocalActor) (LocalVariables|GetGCParams))
  (GameplayCue|AddGameplayCueOnActor(Looping) (LocalVariables|GetLocalActor) "(TagName=\"GameplayCue.ShockLoop\")" (LocalVariables|GetGCParams)))

(fn RemoveGameplayCuefromAddtionalActor
  (params (Actor :type Actor%20Object%20Reference))
  (LocalVariables|SetLocalActor Actor)
  (if (.ReturnValue (Utilities|Map|Find (Variables|Electrocute|GetAddtionalActorToGCParams) (LocalVariables|GetLocalActor)))
    (GameplayCue|RemoveGameplayCueOnActor(Looping) (LocalVariables|GetLocalActor) "(TagName=\"GameplayCue.ShockLoop\")" (.Value (Utilities|Map|Find (Variables|Electrocute|GetAddtionalActorToGCParams) (LocalVariables|GetLocalActor))))))

(fn ApplyDamage
  (bind _returnvalue (Ability|GetAbilitySystemComponentfromActorInfo))
  (bind _hitactor (Variables|Default|GetHitActor))
  (bind _returnvalue_2 (Ability|GetAbilitySystemComponent _hitactor))
  (Ability|HasAuthority
    (:True
      (bind _returnvalue_3 (Ability|GameplayEffect|AssignTagSetbyCallerMagnitude (GameplayEffects|MakeOutgoingSpec _returnvalue (Variables|Default|GetDamageEffectClass) (Math|Conversions|ToFloat(Integer) (Ability|GetAbilityLevel)) (GameplayEffects|MakeEffectContext _returnvalue)) "(TagName=\"Damage.Lightning\")" (Class|AuraDamageGameplayAbility|GetDamagebyAbilityLevel)))
      (LocalVariables|SetDamageSpecHandle _returnvalue_3)
      (GameplayEffects|ApplyGameplayEffectSpecToTarget (Ability|GetAbilitySystemComponentfromActorInfo) (LocalVariables|GetDamageSpecHandle) _returnvalue_2)
      (Development|PrintString (Utilities|GetDisplayName _returnvalue_2))
      (for _array_element (Variables|Electrocute|GetAdditional%20Actors)
        (GameplayEffects|ApplyGameplayEffectSpecToTarget (Ability|GetAbilitySystemComponentfromActorInfo) (LocalVariables|GetDamageSpecHandle) (Ability|GetAbilitySystemComponent _array_element))))))

(fn ApplyDebuff
  (Ability|HasAuthority
    (:True
      (if (Utilities|DoesObjectImplementInterface (Variables|Default|GetHitActor) "/Script/Aura.CombatInterface")
        (Class|AuraAbilitySystemLibrary|ApplyDamageEffect (Class|AuraDamageGameplayAbility|MakeDamageEffectParamfromClassDefaults (Variables|Default|GetHitActor) "0, 0, 0" false))
        (for _array_element (Variables|Electrocute|GetAdditional%20Actors)
          (Class|AuraAbilitySystemLibrary|ApplyDamageEffect (Class|AuraDamageGameplayAbility|MakeDamageEffectParamfromClassDefaults _array_element "0, 0, 0" false)))))))