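; GA_SummonAbility is an enemy gameplay ability that summons random minions around its avatar, using the shaman summon montage.
; It shuffles the generated spawn locations, shows a ground effect at each and plays the montage.
; On the montage's attack event, a delayed loop spawns one minion with a default controller per location.
; Spawning raises the avatar's minion count through an interface message, and each minion's destruction lowers it.
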(event Custom|OnDestroyed_Event
  (params (DestroyedActor :type Actor%20Object%20Reference))
  (Class|CombatInterface|IncreaseMinionCount(Message) (Ability|GetAvatarActorfromActorInfo) -1))

(event Ability|EventActivateAbility
  (bind _returnvalue (Ability|GetAvatarActorfromActorInfo))
  (Variables|Default|SetLocationIndex 0)
  (bind _returnvalue_2 (Class|AuraSummonAbility|GetSpawnLocations))
  (bind _output_get (Variables|Default|SetSpawnLocationArray _returnvalue_2))
  (Utilities|Array|Shuffle _output_get)
  (for _array_element _output_get
    (Niagara|SpawnSystematLocation "/Game/Assets/Effects/Combat/NS_GroundSummon.NS_GroundSummon" _array_element)
    (|PlayMontageandWaitProxy "None" "/Game/Assets/Enemies/Shaman/Animations/AM_Shaman_Summon.AM_Shaman_Summon" 1.0 "None" true 1.0 0.0 false
      (:then
        (Ability|Tasks|WaitGameplayEvent "(TagName=\"Montage.Attack.1\")" 0
          (:EventReceived
            (if (< (Variables|Default|GetLocationIndex) (Utilities|Array|Length (Variables|Default|GetSpawnLocationArray))) :!label _label
              (bind _returnvalue_3 (Game|SpawnActorfromClass (Class|AuraSummonAbility|GetRandomMinionClass) (Math|Transform|MakeTransform (+ (Utilities|Array|Get(acopy) (Variables|Default|GetSpawnLocationArray) (Variables|Default|GetLocationIndex)) "0.000000,0.000000,60.000000") (Transformation|GetActorRotation _returnvalue) "1.000000,1.000000,1.000000") "AlwaysSpawn" "OverrideRootScale" _returnvalue 0))
              (Game|BindEventtoOnDestroyed _returnvalue_3 (delegate Custom|OnDestroyed_Event))
              (Pawn|SpawnDefaultController _returnvalue_3)
              (Class|CombatInterface|IncreaseMinionCount(Message) (Ability|GetAvatarActorfromActorInfo) 1)
              (Math|Integer|IncrementInt (Variables|Default|GetLocationIndex)
                (:%20%20
                  (Utilities|FlowControl|Delay 0.2)
                  (goto _label))))))))))

(event Ability|EventOnEndAbility
  (params (bWasCancelled :type Boolean)))