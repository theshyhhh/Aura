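; Enemy ranged attack ability that fires a projectile at the avatar's combat target.
; On activation it faces the target, then plays a random tagged attack montage from the avatar.
; A gameplay event matching the montage's socket tag triggers the projectile spawn, aimed slightly above the target's current location.
; The ability ends when the montage completes, is interrupted or cancelled, or immediately without a valid target.
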(event Ability|EventActivateAbility
  (bind _returnvalue (Ability|GetAvatarActorfromActorInfo))
  (bind _returnvalue_2 (Class|EnemyInterface|GetCombatTarget(Message) _returnvalue))
  (Utilities|IsValid _returnvalue_2
    (:Is%20Valid
      (bind _ascombat_interface (Utilities|Casting|CastToCombatInterface _returnvalue))
      (Class|CombatInterface|SetFacingTarget _ascombat_interface (Transformation|GetActorLocation _returnvalue_2))
      (bind _returnvalue_3 (Class|CombatInterface|GetAttackMontages(Message) (Ability|GetAvatarActorfromActorInfo)))
      (bind _output_get (Variables|Default|SetTaggedMontage (.OutItem (Utilities|Array|Random _returnvalue_3))))
      (|PlayMontageandWaitProxy "None" (.Montage (Utilities|Struct|BreakTaggedMontage _output_get)) 1.0 "None" true 1.0 0.0 false
        (:then
          (Ability|Tasks|WaitGameplayEvent (.SocketTag (Utilities|Struct|BreakTaggedMontage (Variables|Default|GetTaggedMontage))) 0 true
            (:EventReceived
              (Class|CombatInterface|GetCombatSocketLocation(Message) (Ability|GetAvatarActorfromActorInfo) (.SocketTag (Utilities|Struct|BreakTaggedMontage (Variables|Default|GetTaggedMontage))))
              (bind _returnvalue_4 (Class|EnemyInterface|GetCombatTarget(Message) (Ability|GetAvatarActorfromActorInfo)))
              (Class|AuraProjectileSpell|SpawnProjectile (+ (Transformation|GetActorLocation _returnvalue_4) "0.000000,0.000000,50.000000") (.SocketTag (Utilities|Struct|BreakTaggedMontage (Variables|Default|GetTaggedMontage)))))))
        (:OnCompleted
          (Ability|EndAbility :!label _label))
        (:OnInterrupted
          (goto _label))
        (:OnCancelled
          (goto _label))))
    (:Is%20Not%20Valid
      (Ability|EndAbility))))

(event Ability|EventOnEndAbility
  (params (bWasCancelled :type Boolean)))