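; Base pickup actor that animates itself with a rise on spawn followed by an idle rotate-and-sine motion.
; On BeginPlay, a Timeline curve scaled by MaxHeight offsets the actor vertically from InitialLocation.
; When the Timeline finishes, it sets StartSineMovement, which lets Tick call RotateAndSineMove every frame.
; The graph contains no overlap or collection logic.
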(event EventBeginPlay
  (bind _newtrack_0 (Timeline|Timeline Play)
    (:Update
      (Transformation|SetActorLocation (+ (Math|Vector|MakeVector 0.0 0.0 (* _newtrack_0 (Variables|Default|GetMaxHeight))) (Variables|Default|GetInitialLocation)) false false))
    (:Finished
      (Variables|Default|SetStartSineMovement true))))

(event Collision|EventActorBeginOverlap
  (params (OtherActor :type Actor%20Object%20Reference)))

(event EventTick
  (params (DeltaSeconds :type Float%20%28single-precision%29))
  (if (Variables|Default|GetStartSineMovement)
    (Class|AuraEffectActor|RotateandSineMove DeltaSeconds)))

(fn ConstructionScript)