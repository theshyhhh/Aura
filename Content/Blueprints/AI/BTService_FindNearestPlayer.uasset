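; Behavior tree service that finds the nearest opposing target for the controlled pawn on each AI tick.
; It picks the target tag from the pawn's own tag, so Player-tagged pawns seek Enemy actors and all others seek Player actors.
; It linearly scans all actors with that tag, then writes the closest one and its distance to blackboard keys, even when none is found.
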(event EventReceiveTickAI
  (params (OwnerController :type AI%20Controller%20Object%20Reference) (ControlledPawn :type Pawn%20Object%20Reference) (DeltaSeconds :type Float%20%28single-precision%29))
  (CallFunction|SetTargetTag ControlledPawn)
  (CallFunction|FindNearestTarget ControlledPawn))

(fn SetTargetTag
  (params (Controlled%20Pawn :type Actor%20Object%20Reference))
  (if (Actor|ActorHasTag Controlled%20Pawn "Player")
    (Variables|Default|SetTargetTag "Enemy")
    (else
      (Variables|Default|SetTargetTag "Player"))))

(fn FindNearestTarget
  (params (ControlledPawn :type Pawn%20Object%20Reference))
  (LocalVariables|SetClosestActor 0)
  (LocalVariables|SetClosestDistance 1e+05)
  (bind _outactors (Actor|GetAllActorswithTag (Variables|Default|GetTargetTag)))
  (for _array_element _outactors
    (Utilities|IsValid _array_element
      (:Is%20Valid
        (Utilities|IsValid ControlledPawn
          (:Is%20Valid
            (if (< (Transformation|GetDistanceTo ControlledPawn _array_element) (LocalVariables|GetClosestDistance))
              (LocalVariables|SetClosestActor _array_element)
              (LocalVariables|SetClosestDistance (Transformation|GetDistanceTo ControlledPawn _array_element))))))))
  (Class|BTFunctionLibrary|SetBlackboardValueasObject (Variables|Default|GetTargetToFollow_Selector) (LocalVariables|GetClosestActor))
  (Class|BTFunctionLibrary|SetBlackboardValueasFloat (Variables|Default|GetDistanceToTarget_Selector) (LocalVariables|GetClosestDistance)))